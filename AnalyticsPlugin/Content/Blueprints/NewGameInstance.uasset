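; Game instance that starts an analytics session on Init and holds session and user identifiers.
; Init calls StartSession with a hardcoded name and prints a confirmation when it succeeds.
; InitAnalytics stores the SessionId and UserId passed to it and returns true, while two getters expose those values; Init itself does not set them.
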(event `self.ReceiveInit`
  (bind _result (`/AnalyticsLite/BPFL_Analytics.StartSession` "gino"))
  (if _result
    (`KismetSystemLibrary.PrintString` "AN Session started...")))

(fn `GetSessionId`
  (returns (SessionId :type String))
  (return (`self.Session Id`)))

(fn `GetUserId`
  (returns (UserId :type String))
  (return (`self.User Id`)))

(fn `InitAnalytics`
  (params (SessionId :type String) (UserId :type String))
  (returns (Result :type Boolean))
  (set `self.Session Id` SessionId)
  (set `self.User Id` UserId)
  (return true))