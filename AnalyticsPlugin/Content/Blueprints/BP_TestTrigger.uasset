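; BP_TestTrigger is a test trigger volume that records an event when the first player's pawn enters its box.
; On box overlap it calls RecordEvent with its display name plus a ".BeginOverlap" suffix and the pawn's location and rotation.
; A callback prints the response content and code of the resulting request to show the outcome.
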(event `self.Box.OnComponentBeginOverlap`
  (params (OverlappedComponent :type "PrimitiveComponent Object Reference") (OtherActor :type "Actor Object Reference") (OtherComp :type "PrimitiveComponent Object Reference") (OtherBodyIndex :type Integer) (bFromSweep :type Boolean) (SweepResult :type "HitResult Structure (by ref)"))
  (bind (_returnvalue_location _returnvalue_rotation) (`KismetMathLibrary.BreakTransform` (`self.GetTransform` (`GameplayStatics.GetPlayerPawn` 0))))
  (if (== OtherActor (`GameplayStatics.GetPlayerPawn` 0))
    (`/AnalyticsLite/BPFL_Analytics.RecordEvent` (`KismetStringLibrary.Concat_StrStr` (`KismetSystemLibrary.GetDisplayName` self) ".BeginOverlap") _returnvalue_location _returnvalue_rotation (delegate `-Callback`))))

(event `-Callback`
  (params (Request :type "VaRestRequestJSON Object Reference"))
  (bind _returnvalue (`VaRestRequestJSON.GetResponseContentAsString` Request true))
  (`KismetSystemLibrary.PrintString` _returnvalue)
  (`KismetSystemLibrary.PrintString` (`KismetStringLibrary.Conv_IntToString` (`VaRestRequestJSON.GetResponseCode` Request))))

(fn `UserConstructionScript`)